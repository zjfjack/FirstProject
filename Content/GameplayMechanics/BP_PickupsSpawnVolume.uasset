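; Pickup spawn volume that spawns one actor shortly after play begins.
; BeginPlay waits briefly, then passes the results of GetSpawnActor and GetSpawnPoint to SpawnActor.
; The SpawnActor override plays a gold sparkle particle effect at the location, then calls the parent implementation to do the spawn.
; An earlier Blueprint-only spawn node remains in the graph, unconnected.
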(event EventBeginPlay
  (Utilities|FlowControl|Delay 0.2)
  (Class|SpawnVolume|SpawnActor (Class|SpawnVolume|GetSpawnActor) (Class|SpawnVolume|GetSpawnPoint)))

(event EventSpawnActor
  (params (ToSpawn :type Object%20Class%20Reference) (Location :type Vector%20%28by%20ref%29 :default "0, 0, 0"))
  (Effects|SpawnEmitteratLocation "/Game/InfinityBladeEffects/Effects/FX_Treasure/Gold_Bag/P_GoldSparkle_Bag_Pickup.P_GoldSparkle_Bag_Pickup" Location)
  (|CallParentFunction ToSpawn Location))

(fn ConstructionScript)