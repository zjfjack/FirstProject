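; BP_MainCharacter is the main character Blueprint, handling the loading of a weapon by name.
; The LoadWeapon event maps the name to one of four weapon Blueprint classes through GetWeaponClass.
; It then spawns that weapon at SpawnWeaponTransform and calls Equip on it, passing the character itself.
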(event EventLoadWeapon
  (params (WeaponName :type String))
  ;[1 1 1] Load Weapon Event
  (bind _weaponclass (CallFunction|GetWeaponClass WeaponName))
  (bind _returnvalue (Game|SpawnActorfromClass _weaponclass (Variables|Default|GetSpawnWeaponTransform) "Undefined" 0 0))
  (Class|Weapon|Equip _returnvalue self))

(fn ConstructionScript)

(fn GetWeaponClass
  (params (WeaponName :type String))
  (switch string WeaponName
    (:Glimmer
      (return "/Game/Weapons/BP_WeaponGlimmer.BP_WeaponGlimmer_C"))
    (:FissureBlade
      (return "/Game/Weapons/BP_WeaponFissureBlade.BP_WeaponFissureBlade_C"))
    (:DragonSword
      (return "/Game/Weapons/BP_WeaponDragonSword.BP_WeaponDragonSword_C"))
    (:GreatBlade
      (return "/Game/Weapons/BP_WeaponGreatBlade.BP_WeaponGreatBlade_C"))))